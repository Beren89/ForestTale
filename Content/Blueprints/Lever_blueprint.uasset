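; Interactable lever that sends positive or negative trigger messages to a target when pulled to either end.
; Interact rotates the arm by the look-up input, with an upper box and lower sphere overlap acting as limit stops.
; Reaching a stop clears the character's InteractionActive, messages the target and calls the matching trigger-activated event.
; BeginPlay applies the configurable meshes, and Highlight/Lowlight toggle a point light.
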(event OnComponentEndOverlap(DownSphere)
  (params (OtherActor :type Actor%20Object%20Reference) (OtherComp :type Primitive%20Component%20Object%20Reference) (OtherBodyIndex :type Integer))
  ;[1 1 1] Reset Box hit
  (if (== OtherComp (Variables|Default|GetLever_arm))
    (Variables|Default|SetSphereHit false)))

(event OnComponentEndOverlap(UpBox)
  (params (OtherActor :type Actor%20Object%20Reference) (OtherComp :type Primitive%20Component%20Object%20Reference) (OtherBodyIndex :type Integer))
  ;[1 1 1] Reset Box hit
  (if (== OtherComp (Variables|Default|GetLever_arm))
    (Variables|Default|SetBoxHit false)))

(event OnComponentBeginOverlap(UpBox)
  (params (OtherActor :type Actor%20Object%20Reference) (OtherComp :type Primitive%20Component%20Object%20Reference) (OtherBodyIndex :type Integer) (bFromSweep :type Boolean) (SweepResult :type Hit%20Result%20Structure%20%28by%20ref%29))
  ;[1 1 1] Activating Trigger Interface
  (if (== OtherComp (Variables|Default|GetLever_arm))
    (bind _asthird_person_character (Utilities|Casting|CastToThirdPersonCharacter (Game|GetPlayerCharacter 0)))
    (Variables|/Game/Blueprints/ThirdPersonCharacter.ThirdPersonCharacter_C|SetInteraction%20Active _asthird_person_character false)
    (Class|Triggers|TriggerPositive(Message) (Variables|Default|GetTarget) 0.0)
    (Default|CallPositiveTriggerActivated)
    (Variables|Default|SetBoxHit true)))

(event OnComponentBeginOverlap(DownSphere)
  (params (OtherActor :type Actor%20Object%20Reference) (OtherComp :type Primitive%20Component%20Object%20Reference) (OtherBodyIndex :type Integer) (bFromSweep :type Boolean) (SweepResult :type Hit%20Result%20Structure%20%28by%20ref%29))
  ;[1 1 1] Activating Trigger Interface
  (if (== OtherComp (Variables|Default|GetLever_arm))
    (bind _asthird_person_character (Utilities|Casting|CastToThirdPersonCharacter (Game|GetPlayerCharacter 0)))
    (Variables|/Game/Blueprints/ThirdPersonCharacter.ThirdPersonCharacter_C|SetInteraction%20Active _asthird_person_character false)
    (Class|Triggers|TriggerNegative(Message) (Variables|Default|GetTarget) 0.0)
    (Default|CallNegativeTriggerActivated)
    (Variables|Default|SetSphereHit true)))

(event EventBeginPlay
  ;[1 1 1] Setting Lever and Secondary Meshes
  (Components|StaticMesh|SetStaticMesh (Variables|Default|GetArmMeshComponent) (Variables|Default|GetArmMeshVariable))
  (Components|StaticMesh|SetStaticMesh (Variables|Default|GetSecondaryMeshComponent) (Variables|Default|GetSecondaryMeshVariable)))

(event EventInteract
  (bind _returnvalue (Input|AxisValues|GetLookUp))
  ;[1 1 1] Lever rotation
  (bind _asthird_person_character (Utilities|Casting|CastToThirdPersonCharacter (Game|GetPlayerCharacter 0)))
  (Variables|/Game/Blueprints/ThirdPersonCharacter.ThirdPersonCharacter_C|SetRotation%20Active _asthird_person_character true)
  (if (Variables|Default|GetBoxHit)
    (if (< _returnvalue 0.0)
      (Transformation|AddLocalRotation (Variables|Default|GetLever_arm) (Math|Rotator|MakeRotator 0.0 (* -1 _returnvalue) 0.0) false false :!label _label))
    (elif (Variables|Default|GetSphereHit)
      (if (> _returnvalue 0.0)
        (goto _label))
      (else
        (goto _label)))))

(event EventHighlight
  (Rendering|SetVisibility (Variables|Default|GetPointLight) true false))

(event EventLowlight
  (Rendering|SetVisibility (Variables|Default|GetPointLight) false false))

(fn ConstructionScript)