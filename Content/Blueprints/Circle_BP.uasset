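; Circle_BP is an interactable rotating piece for a circle puzzle, with a configurable arm mesh and a point light for highlighting.
; Until the puzzle is marked done, interacting sets the player character's rotation flag, yaws the LeverArm by the inverted turn value and fires a positive trigger.
; Stopping interaction fires the negative trigger.
; UpBox overlaps with DownSphere tell a target when the circle's position becomes correct or is undone.
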(event OnComponentEndOverlap(UpBox)
  (params (OtherActor :type Actor%20Object%20Reference) (OtherComp :type Primitive%20Component%20Object%20Reference) (OtherBodyIndex :type Integer))
  ;[1 1 1] Activating Trigger Interface
  (if (== OtherComp (Variables|Default|GetDown%20Sphere))
    (Class|PuzzlesInterface|CirclePositionUndone(Message) (Variables|Default|GetTarget))))

(event OnComponentBeginOverlap(UpBox)
  (params (OtherActor :type Actor%20Object%20Reference) (OtherComp :type Primitive%20Component%20Object%20Reference) (OtherBodyIndex :type Integer) (bFromSweep :type Boolean) (SweepResult :type Hit%20Result%20Structure%20%28by%20ref%29))
  ;[1 1 1] Activating Trigger Interface
  (if (== OtherComp (Variables|Default|GetDown%20Sphere))
    (Class|PuzzlesInterface|CirclePositionDone(Message) (Variables|Default|GetTarget))))

(event EventBeginPlay
  ;[1 1 1] Setting Lever and Secondary Meshes
  (Components|StaticMesh|SetStaticMesh (Variables|Default|GetArmMeshComponent) (Variables|Default|GetArmMeshVariable)))

(event EventInteract
  ;[1 1 1] Lever rotation
  (if (not (Variables|Default|GetDone))
    (bind _asthird_person_character (Utilities|Casting|CastToThirdPersonCharacter (Game|GetPlayerCharacter 0)))
    (Variables|/Game/Blueprints/ThirdPersonCharacter.ThirdPersonCharacter_C|SetRotation%20Active _asthird_person_character true)
    (Transformation|AddLocalRotation (Variables|Default|GetLever_arm) (Math|Rotator|MakeRotator 0.0 0.0 (* -1 (Input|AxisValues|GetTurn))) false false)
    (Default|CallPositiveTriggerActivated)))

(event EventHighlight
  ;[1 1 1] Highlight
  (Rendering|SetVisibility (Variables|Default|GetPointLight) true false))

(event EventLowlight
  ;[1 1 1] Highlight
  (Rendering|SetVisibility (Variables|Default|GetPointLight) false false))

(event EventStopInteraction
  ;[1 1 1] Lever rotation
  (Default|CallNegativeTriggerActivated))

(event EventCirclePuzzleDone
  ;[1 1 1] Lever rotation
  (Variables|Default|SetDone true))

(fn ConstructionScript
  (Components|StaticMesh|SetStaticMesh (Variables|Default|GetArmMeshComponent) (Variables|Default|GetArmMeshVariable)))