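; MovableObj is a movable mesh object Blueprint with a point light that serves as its highlight.
; Highlight and Lowlight events show and hide the light.
; Tick turns overlap event generation back on for the static mesh whenever it is off.
; Any hit switches off physics simulation on the mesh.
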(event Collision|EventHit
  (params (MyComp :type Primitive%20Component%20Object%20Reference) (Other :type Actor%20Object%20Reference) (OtherComp :type Primitive%20Component%20Object%20Reference) (bSelfMoved :type Boolean) (HitLocation :type Vector :default "0, 0, 0") (HitNormal :type Vector :default "0, 0, 0") (NormalImpulse :type Vector :default "0, 0, 0") (Hit :type Hit%20Result%20Structure%20%28by%20ref%29))
  (Physics|SetSimulatePhysics (Variables|Debug|GetStaticMeshComponent) false))

(event EventTick
  (params (DeltaSeconds :type Float%20%28single-precision%29))
  (bind _staticmeshcomponent (Variables|Debug|GetStaticMeshComponent))
  (if (not (Variables|/Script/Engine.PrimitiveComponent|GetbGenerateOverlapEvents _staticmeshcomponent))
    (Variables|/Script/Engine.PrimitiveComponent|SetbGenerateOverlapEvents _staticmeshcomponent true)))

(event EventHighlight
  (Rendering|SetVisibility (Variables|Default|GetPointLight) true false))

(event EventLowlight
  (Rendering|SetVisibility (Variables|Default|GetPointLight) false false))

(fn ConstructionScript)