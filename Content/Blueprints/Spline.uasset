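; Spline actor Blueprint that builds a deformed mesh along an editable spline, with no runtime logic.
; The construction script adds one spline mesh component per segment, using a configurable mesh, material and material slot.
; Each segment takes its start and end positions and tangents from neighboring spline points.
; Per-point Y/Z scale drives the segment's end scales, and point roll divided by a constant drives its twist.
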(event EventBeginPlay)

(event EventActorBeginOverlap
  (params (OtherActor :type Actor%20Object%20Reference)))

(event EventTick
  (params (DeltaSeconds :type Float%20%28single-precision%29)))

(fn ConstructionScript
  (bind _spline (Variables|Default|GetSpline))
  (bind _spline_2 (Variables|Default|GetSpline))
  (for _index (range 0 (- (Spline|GetNumberOfSplinePoints _spline_2) 2))
    (bind _returnvalue (AddComponent|AddSplineMeshComponent true))
    (bind _output_get (Variables|Default|SetSplineSection _returnvalue))
    (Components|StaticMesh|SetStaticMesh _output_get (Variables|Default|GetSplineMesh))
    (Rendering|Material|SetMaterial _output_get (Variables|Default|GetSplineMatIndex) (Variables|Default|GetSplineMaterial))
    (SplineMesh|SetEndScale _output_get (Math|Vector2D|MakeVector2D (.Y (Math|Vector|BreakVector (Spline|GetScaleatSplinePoint _spline_2 (+ _index 1)))) (.Z (Math|Vector|BreakVector (Spline|GetScaleatSplinePoint _spline_2 (+ _index 1))))) :!class /Script/Engine.SplineMeshComponent)
    (SplineMesh|SetStartScale _output_get (Math|Vector2D|MakeVector2D (.Y (Math|Vector|BreakVector (Spline|GetScaleatSplinePoint _spline_2 _index))) (.Z (Math|Vector|BreakVector (Spline|GetScaleatSplinePoint _spline_2 _index)))) :!class /Script/Engine.SplineMeshComponent)
    (Class|SplineMeshComponent|SetStartRoll (Variables|Default|GetSplineSection) (/ (.Roll (Math|Rotator|BreakRotator (Spline|GetRotationatSplinePoint _spline _index "Local"))) 1.3e+02))
    (Class|SplineMeshComponent|SetEndRoll (Variables|Default|GetSplineSection) (/ (.Roll (Math|Rotator|BreakRotator (Spline|GetRotationatSplinePoint _spline (+ _index 1) "Local"))) 1.3e+02))
    (Class|SceneComponent|Attachto (Variables|Default|GetSplineSection) (Variables|Default|GetSpline) "None" "KeepRelativeOffset" true)
    (SplineMesh|SetStartandEnd (Variables|Default|GetSplineSection) (.Location (Spline|GetLocationandTangentatSplinePoint _spline _index "Local")) (.Tangent (Spline|GetLocationandTangentatSplinePoint _spline _index "Local")) (.Location (Spline|GetLocationandTangentatSplinePoint _spline (+ _index 1) "Local")) (.Tangent (Spline|GetLocationandTangentatSplinePoint _spline (+ _index 1) "Local")) :!class /Script/Engine.SplineMeshComponent)))