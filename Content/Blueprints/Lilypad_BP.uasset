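; Lilypad actor that gives the player low gravity and a far zoomed-out camera when stepped on.
; Begin overlap on CharacterCheck sets both effects and resets a DoOnce fed by Tick; end overlap clears the stepped-on flag.
; The DoOnce output checks whether the player has left the pad and is not falling before restoring gravity and camera distance.
; Highlight and Lowlight events toggle the pad's point light.
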(event OnComponentEndOverlap(CharacterCheck)
  (params (OtherActor :type Actor%20Object%20Reference) (OtherComp :type Primitive%20Component%20Object%20Reference) (OtherBodyIndex :type Integer))
  (if (== OtherActor (Game|GetPlayerCharacter 0))
    (Variables|Default|SetStepped%20on%20Lily false)))

(event OnComponentBeginOverlap(CharacterCheck)
  (params (OtherActor :type Actor%20Object%20Reference) (OtherComp :type Primitive%20Component%20Object%20Reference) (OtherBodyIndex :type Integer) (bFromSweep :type Boolean) (SweepResult :type Hit%20Result%20Structure%20%28by%20ref%29))
  (bind _returnvalue (Game|GetPlayerCharacter 0))
  (if (== OtherActor _returnvalue)
    (Variables|Default|SetStepped%20on%20Lily true)
    (bind _asthird_person_character (Utilities|Casting|CastToThirdPersonCharacter _returnvalue))
    (Variables|/Script/Engine.CharacterMovementComponent|SetGravityScale (Variables|/Script/Engine.Character|GetCharacterMovement _asthird_person_character) 0.2)
    (Variables|/Script/Engine.SpringArmComponent|SetTargetArmLength (Variables|/Game/Blueprints/ThirdPersonCharacter.ThirdPersonCharacter_C|GetSpringArm _asthird_person_character) 3e+03)
    (Utilities|FlowControl|DoOnce true) ; enters at Reset
  ))

(event EventTick
  (params (DeltaSeconds :type Float%20%28single-precision%29))
  (Utilities|FlowControl|DoOnce true
    (:Completed
      (if (not (Variables|Default|GetStepped%20on%20Lily))
        (if (AI|Components|NavMovement|IsFalling (Variables|/Script/Engine.Character|GetCharacterMovement (stale OnComponentBeginOverlap(CharacterCheck) _asthird_person_character)))
          (bind _asthird_person_character (Utilities|Casting|CastToThirdPersonCharacter (Game|GetPlayerCharacter 0)))
          (else
            (Variables|/Script/Engine.CharacterMovementComponent|SetGravityScale (Variables|/Script/Engine.Character|GetCharacterMovement _asthird_person_character) 1.0)
            (Variables|/Game/Blueprints/ThirdPersonCharacter.ThirdPersonCharacter_C|SetGravity%20Reset _asthird_person_character true)
            (Variables|/Script/Engine.SpringArmComponent|SetTargetArmLength (Variables|/Game/Blueprints/ThirdPersonCharacter.ThirdPersonCharacter_C|GetSpringArm _asthird_person_character) 5e+02)))))))

(event EventHighlight
  (Rendering|SetVisibility (Variables|Default|GetPointLight) true false))

(event EventLowlight
  (Rendering|SetVisibility (Variables|Default|GetPointLight) false false))

(fn ConstructionScript)