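; Shrine control Blueprint that tracks completion of a circle puzzle.
; CirclePositionDone and CirclePositionUndone raise or lower a CirclePuzzleStatus counter, then both run CheckCompletion.
; When the counter equals four, it calls CirclePuzzleDoneMessage on the Circles reference and sets PuzzleComplete, which is never cleared here.
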(event Custom|Check%20Completion
  (if (== 4 (Variables|Default|GetCirclePuzzleStatus))
    (Class|PuzzlesInterface|CirclePuzzleDone(Message) (Variables|Default|GetCircles))
    (Variables|Default|SetPuzzleComplete true)))

(event EventCirclePositionDone
  (Variables|Default|SetCirclePuzzleStatus (+ (Variables|Default|GetCirclePuzzleStatus) 1))
  (CallFunction|CheckCompletion))

(event EventCirclePositionUndone
  (Variables|Default|SetCirclePuzzleStatus (- (Variables|Default|GetCirclePuzzleStatus) 1))
  (CallFunction|CheckCompletion))

(fn ConstructionScript)