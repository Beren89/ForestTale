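; Pond spring actor that raises or lowers itself when triggered and signals three target actors when a rock rests in it.
; PondRock overlaps on its Box send TriggerPositive to the targets, and leaving sends TriggerNegative, through a trigger interface.
; Lilypad overlaps toggle the Cube's collision.
; Received triggers set a goal one increment from the current height, which Tick eases toward with FInterpTo.
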(event OnComponentBeginOverlap(Box)
  (params (OtherActor :type Actor%20Object%20Reference) (OtherComp :type Primitive%20Component%20Object%20Reference) (OtherBodyIndex :type Integer) (bFromSweep :type Boolean) (SweepResult :type Hit%20Result%20Structure%20%28by%20ref%29))
  ;[1 1 1] Overlapping check
  (if (Actor|ActorHasTag OtherActor "Lilypad")
    (Collision|SetCollisionEnabled (Variables|Default|GetCube) "QueryAndPhysics")
    (elif (Actor|ActorHasTag OtherActor "PondRock")
      (CallFunction|TriggerPositive (Variables|Default|GetTargetArray) (Variables|Default|GetOutboundIncrement01)))))

(event OnComponentEndOverlap(Box)
  (params (OtherActor :type Actor%20Object%20Reference) (OtherComp :type Primitive%20Component%20Object%20Reference) (OtherBodyIndex :type Integer))
  ;[1 1 1] Overlapping check
  (if (Actor|ActorHasTag OtherActor "Lilypad")
    (Collision|SetCollisionEnabled (Variables|Default|GetCube) "NoCollision")
    (elif (Actor|ActorHasTag OtherActor "PondRock")
      (CallFunction|TriggerNegative (Variables|Default|GetTargetArray) (Variables|Default|GetOutboundIncrement01)))))

(event Custom|IncreseHeight
  (bind _defaultsceneroot (Variables|Default|GetDefaultSceneRoot))
  (bind _returnvalue (Transformation|GetWorldLocation _defaultsceneroot))
  (bind (_x _y _z) (Math|Vector|BreakVector _returnvalue))
  ;[1 1 1] Height increasing
  (Transformation|SetWorldLocation (Variables|Default|GetDefaultSceneRoot) (Math|Vector|MakeVector _x _y (Math|Interpolation|FInterpTo (Variables|Default|GetTransitientHeightPosition) (+ (Variables|Default|GetSprout%20Height) (Variables|Default|GetIncrement)) (Utilities|Time|GetWorldDeltaSeconds) 5.0)) false false)
  (Variables|Default|SetTransitientHeightPosition (Math|Interpolation|FInterpTo (Variables|Default|GetTransitientHeightPosition) (+ (Variables|Default|GetSprout%20Height) (Variables|Default|GetIncrement)) (Utilities|Time|GetWorldDeltaSeconds) 5.0))
  (if (Math|Float|NearlyEqual(Float) _z (+ (Variables|Default|GetSprout%20Height) (Variables|Default|GetIncrement)) 0.1)
    (Variables|Default|SetSprout%20Height _z)
    (Development|PrintString "CHECK")
    (Variables|Default|SetMoveUp false)))

(event Custom|DecreseHeight
  (bind _defaultsceneroot (Variables|Default|GetDefaultSceneRoot))
  (bind _returnvalue (Transformation|GetWorldLocation _defaultsceneroot))
  (bind (_x _y _z) (Math|Vector|BreakVector _returnvalue))
  ;[1 1 1] Height Decreasing
  (Transformation|SetWorldLocation (Variables|Default|GetDefaultSceneRoot) (Math|Vector|MakeVector _x _y (Math|Interpolation|FInterpTo (Variables|Default|GetTransitientHeightPosition) (- (Variables|Default|GetSprout%20Height) (Variables|Default|GetIncrement)) (Utilities|Time|GetWorldDeltaSeconds) 5.0)) false false)
  (Variables|Default|SetTransitientHeightPosition (Math|Interpolation|FInterpTo (Variables|Default|GetTransitientHeightPosition) (- (Variables|Default|GetSprout%20Height) (Variables|Default|GetIncrement)) (Utilities|Time|GetWorldDeltaSeconds) 5.0))
  (if (Math|Float|NearlyEqual(Float) _z (- (Variables|Default|GetSprout%20Height) (Variables|Default|GetIncrement)) 0.1)
    (Variables|Default|SetSprout%20Height _z)
    (Development|PrintString "CHECK")
    (Variables|Default|SetMoveDown false)))

(event EventTriggerPositive
  (params (Increment :type Float%20%28single-precision%29))
  ;[1 1 1] Trigger Interface Events
  (Variables|Default|SetIncrement Increment)
  (bind _output_get (Variables|Default|SetSprout%20Height (.Z (Math|Vector|BreakVector (Transformation|GetWorldLocation (Variables|Default|GetDefaultSceneRoot))))))
  (Variables|Default|SetTransitientHeightPosition _output_get)
  (Variables|Default|SetMoveDown false)
  (Variables|Default|SetMoveUp true))

(event EventTriggerNegative
  (params (Increment :type Float%20%28single-precision%29))
  ;[1 1 1] Trigger Interface Events
  (Variables|Default|SetIncrement Increment)
  (bind _output_get (Variables|Default|SetSprout%20Height (.Z (Math|Vector|BreakVector (Transformation|GetWorldLocation (Variables|Default|GetDefaultSceneRoot))))))
  (Variables|Default|SetTransitientHeightPosition _output_get)
  (Variables|Default|SetMoveUp false)
  (Variables|Default|SetMoveDown true))

(event EventBeginPlay
  ;[1 1 1] Initial setup
  (bind _output_get (Variables|Default|SetInitial%20Sprout%20Height (.Z (Math|Vector|BreakVector (Transformation|GetWorldLocation (Variables|Default|GetDefaultSceneRoot))))))
  (Variables|Default|SetTransitientHeightPosition _output_get)
  (Collision|SetCollisionEnabled (Variables|Default|GetCube) "NoCollision")
  (Variables|Default|SetTargetArray (Utilities|Array|MakeArray (Variables|Default|GetTarget01) (Variables|Default|GetTarget02) (Variables|Default|GetTarget03))))

(event EventTick
  (params (DeltaSeconds :type Float%20%28single-precision%29))
  ;[0 1 0.3078] Tick
  (if (Variables|Default|GetMoveUp)
    (CallFunction|IncreseHeight)
    (elif (Variables|Default|GetMoveDown)
      (CallFunction|DecreseHeight))))

(fn ConstructionScript)