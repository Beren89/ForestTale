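; Particle effect actor that does manual distance-based LOD by switching between three particle components.
; On BeginPlay it copies the main component's instance parameters to the second and third components.
; Every Tick it measures the distance to player character 0 and shows only the near, middle or far component, using two fixed distance thresholds.
; Switching only toggles visibility, without propagating to children.
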(event EventBeginPlay
  (bind _output_get (Variables|/Script/Engine.ParticleSystemComponent|SetInstanceParameters (Variables|Default|GetSecondParticle) (Variables|/Script/Engine.ParticleSystemComponent|GetInstanceParameters (Variables|Emitter|GetParticleSystemComponent))))
  (Variables|/Script/Engine.ParticleSystemComponent|SetInstanceParameters (Variables|Default|GetThirdParticle) _output_get))

(event EventTick
  (params (DeltaSeconds :type Float%20%28single-precision%29))
  (bind _returnvalue (Game|GetPlayerCharacter 0))
  (bind _self self)
  (bind _returnvalue_2 (Transformation|GetDistanceTo _returnvalue _self))
  (if (<= _returnvalue_2 1e+03)
    (Rendering|SetVisibility (Variables|Emitter|GetParticleSystemComponent) true false)
    (Rendering|SetVisibility (Variables|Default|GetSecondParticle) false false)
    (Rendering|SetVisibility (Variables|Default|GetThirdParticle) false false)
    (else
      (Rendering|SetVisibility (Variables|Emitter|GetParticleSystemComponent) false false)
      (if (<= _returnvalue_2 2e+03)
        (Rendering|SetVisibility (Variables|Default|GetSecondParticle) true false)
        (Rendering|SetVisibility (Variables|Default|GetThirdParticle) false false)
        (else
          (Rendering|SetVisibility (Variables|Default|GetThirdParticle) true false)
          (Rendering|SetVisibility (Variables|Default|GetSecondParticle) false false))))))

(fn ConstructionScript)