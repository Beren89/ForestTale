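; Flower sound puzzle controller that plays a four-note tune and checks the sounds sent back to it in order.
; PlayCue plays the notes in sequence at the actor's location with player input disabled.
; TransmitSound advances through the tune on a match and resets to the first note on a mismatch.
; Completing it increments the cycle, loads that cycle's tune and plays it; cycles two to four have no sounds assigned.
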(event Custom|Set%20Tune
  (if (== (Variables|Default|GetCurrentCycle) 1)
    (Variables|Default|SetSound_01 "/Game/Sounds/snd_glass_ping_hiPitch.snd_glass_ping_hiPitch")
    (Variables|Default|SetSound_02 "/Game/Sounds/snd_glass_ping_hiPitch.snd_glass_ping_hiPitch")
    (Variables|Default|SetSound_03 "/Game/Sounds/snd_glass_ping_hiPitch.snd_glass_ping_hiPitch")
    (Variables|Default|SetSound_04 "/Game/Sounds/snd_glass_ping_loPitch.snd_glass_ping_loPitch")
    (elif (== (Variables|Default|GetCurrentCycle) 2)
      (Variables|Default|SetSound_01 0)
      (Variables|Default|SetSound_02 0)
      (Variables|Default|SetSound_03 0)
      (Variables|Default|SetSound_04 0)
      (elif (== (Variables|Default|GetCurrentCycle) 3)
        (Variables|Default|SetSound_01 0)
        (Variables|Default|SetSound_02 0)
        (Variables|Default|SetSound_03 0)
        (Variables|Default|SetSound_04 0)
        (elif (== (Variables|Default|GetCurrentCycle) 4)
          (Variables|Default|SetSound_01 0)
          (Variables|Default|SetSound_02 0)
          (Variables|Default|SetSound_03 0)
          (Variables|Default|SetSound_04 0))))))

(event Custom|Play%20Cue
  (bind _returnvalue (Transformation|GetActorLocation))
  (bind _sound_02 (Variables|Default|GetSound_02))
  (bind _sound_03 (Variables|Default|GetSound_03))
  (bind _sound_04 (Variables|Default|GetSound_04))
  (bind _sound_01 (Variables|Default|GetSound_01))
  (Input|DisableInput (Game|GetPlayerCharacter 0) 0)
  (Audio|PlaySoundatLocation _sound_01 _returnvalue)
  (Utilities|FlowControl|Delay (Variables|/Script/Engine.SoundBase|GetDuration _sound_01))
  (Audio|PlaySoundatLocation _sound_02 _returnvalue)
  (Utilities|FlowControl|Delay (Variables|/Script/Engine.SoundBase|GetDuration _sound_02))
  (Audio|PlaySoundatLocation _sound_03 _returnvalue)
  (Utilities|FlowControl|Delay (Variables|/Script/Engine.SoundBase|GetDuration _sound_03))
  (Audio|PlaySoundatLocation _sound_04 _returnvalue)
  (Utilities|FlowControl|Delay (Variables|/Script/Engine.SoundBase|GetDuration _sound_04))
  (Variables|Default|SetCurrent%20Sound (Variables|Default|GetSound_01))
  (Input|EnableInput (Game|GetPlayerCharacter 0) 0))

(event Custom|Set%20Current%20Sound
  (bind _sound_04 (Variables|Default|GetSound_04))
  (if (== (Variables|Default|GetCurrentPassage) 1)
    (Variables|Default|SetCurrent%20Sound (Variables|Default|GetSound_02))
    (elif (== (Variables|Default|GetCurrentPassage) 2)
      (Variables|Default|SetCurrent%20Sound (Variables|Default|GetSound_03))
      (elif (== (Variables|Default|GetCurrentPassage) 3)
        (Variables|Default|SetCurrent%20Sound _sound_04)
        (elif (== (Variables|Default|GetCurrentPassage) 4)
          (Variables|Default|SetCurrentCycle (+ (Variables|Default|GetCurrentCycle) 1))
          (Utilities|FlowControl|Delay (Variables|/Script/Engine.SoundBase|GetDuration _sound_04))
          (CallFunction|SetTune)
          (CallFunction|PlayCue))))))

(event EventTransmitSound
  (params (Input%20Sound :type Sound%20Base%20Object%20Reference))
  (if (== Input%20Sound (Variables|Default|GetCurrent%20Sound))
    (Variables|Default|SetCurrentPassage (+ (Variables|Default|GetCurrentPassage) 1))
    (CallFunction|SetCurrentSound)
    (else
      (Variables|Default|SetCurrent%20Sound (Variables|Default|GetSound_01))
      (Variables|Default|SetCurrentPassage 0)
      (Development|PrintString "WRONG!"))))

(fn ConstructionScript)